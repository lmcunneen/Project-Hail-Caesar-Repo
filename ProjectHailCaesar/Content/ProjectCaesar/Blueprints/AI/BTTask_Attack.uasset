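; Behavior tree task that makes an enemy attack the player, or taunt if the player is already dead.
; It reads the player character from a blackboard key and checks its IsDead flag to call either Attack or Taunt on the controlled BP_Enemy.
; Both branches wait a fixed delay before finishing the task as successful; a failed cast stops without finishing it.
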(event `self.ReceiveExecuteAI`
  (params (OwnerController :type "AIController Object Reference") (ControlledPawn :type "Pawn Object Reference"))
  (bind _asbp_third_person_character (cast `/Game/ThirdPerson/Blueprints/BP_ThirdPersonCharacter` (`BTFunctionLibrary.GetBlackboardValueAsObject` (`self.PlayerKey`))))
  (if (`/Game/ThirdPerson/Blueprints/BP_ThirdPersonCharacter.IsDead` _asbp_third_person_character)
    (bind _asbp_enemy (cast `/Game/ProjectCaesar/Blueprints/BP_Enemy` ControlledPawn))
    (`/Game/ThirdPerson/Blueprints/BP_ThirdPersonCharacter.Taunt` _asbp_enemy)
    (`KismetSystemLibrary.Delay` 1.0)
    (else
      (bind _asbp_enemy_2 (cast `/Game/ProjectCaesar/Blueprints/BP_Enemy` ControlledPawn))
      (`/Game/ThirdPerson/Blueprints/BP_ThirdPersonCharacter.Attack` _asbp_enemy_2)
      (`KismetSystemLibrary.Delay` 1.0)))
  (`self.FinishExecute` true))