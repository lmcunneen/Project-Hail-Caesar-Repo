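; Attention meter that scores how engaging the player's combat is, with events to play or stop the emperor's waning and uninterested sequences.
; Tick advances timers since kills, fights, hurts, taunts and attacks, prints debug values and applies a boredom penalty when fighting lapses.
; Reported action states enter a ten-entry history that reduces the score for repeats.
; The clamped 0–1000 rating maps to five attention levels.
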(event `StopAllLevelSequences`
  (`MovieSceneSequencePlayer.Stop` (`LevelSequenceActor.SequencePlayer` (`self.WaningSequence`)))
  (`MovieSceneSequencePlayer.Stop` (`LevelSequenceActor.SequencePlayer` (`self.UninterestedSequence`))))

(event `PlayEmperorWaning`
  (bind _sequenceplayer (`LevelSequenceActor.SequencePlayer` (`self.WaningSequence`)))
  (if (not (`MovieSceneSequencePlayer.IsPlaying` _sequenceplayer))
    (`MovieSceneSequencePlayer.Play` _sequenceplayer)))

(event `PlayEmperorUninterested`
  (bind _sequenceplayer (`LevelSequenceActor.SequencePlayer` (`self.UninterestedSequence`)))
  (if (not (`MovieSceneSequencePlayer.IsPlaying` _sequenceplayer))
    (`MovieSceneSequencePlayer.Play` _sequenceplayer)))

(event `self.ReceiveBeginPlay`
  ;[0.05098 0.05098 0.05098] Initialising Player Reference
  (bind _asbp_third_person_character (cast `/Game/ThirdPerson/Blueprints/BP_ThirdPersonCharacter` (`GameplayStatics.GetPlayerPawn` 0)))
  (bind _output_get (set `self.Player` _asbp_third_person_character))
  ;[0.474 0.474 0.474] Run InitialiseAttentionMetrics in Player
  (`/Game/ThirdPerson/Blueprints/BP_ThirdPersonCharacter.IntialiseAttentionMetrics` _output_get self)
  (`self.SetAttentionLevelFromRating`))

(event `self.ReceiveTick`
  (params (DeltaSeconds :type "Float (single-precision)"))
  ;[1 0.3208 0.291] Increment and Display Timers
  (if (not (`self.IsDisabled`))
    (`self.IncrementAllTimers` DeltaSeconds)
    (`self.DisplayMetricsDebug`)
    (`self.OnTickMetricEvaluation`)))

(event `ResetLastKillTimer`
  ;[0.2678 0.5142 1] When called, reset timer and print associated debug log
  (`self.ResetTimeFloat` (`self.TimeFromLastKill`))
  (`KismetSystemLibrary.PrintString` "Last Kill Timer Reset!" true false (struct :`R` 0.109307 :`G` 0.864583 :`B` 0.119964 :`A` 1.0)))

(event `ResetLastFightTimer`
  ;[0.2678 0.5142 1] When called, reset timer and print associated debug log
  (`self.ResetTimeFloat` (`self.TimeFromLastFight`))
  (`KismetSystemLibrary.PrintString` "Last Fight Timer Reset!" true false (struct :`R` 0.109307 :`G` 0.864583 :`B` 0.119964 :`A` 1.0)))

(event `ResetLastPlayerHurtTimer`
  ;[0.2678 0.5142 1] When called, reset timer and print associated debug log
  (`self.ResetTimeFloat` (`self.TimeFromLastPlayerHurt`))
  (`KismetSystemLibrary.PrintString` "Last Player Hurt Timer Reset!" true false (struct :`R` 0.109307 :`G` 0.864583 :`B` 0.119964 :`A` 1.0)))

(event `ResetLastTauntTimer`
  ;[0.2678 0.5142 1] When called, reset timer and print associated debug log
  (`self.ResetTimeFloat` (`self.TimeFromLastTaunt`))
  (`KismetSystemLibrary.PrintString` "Last Taunt Timer Reset!" true false (struct :`R` 0.109307 :`G` 0.864583 :`B` 0.119964 :`A` 1.0)))

(event `EvaluateNewActionState`
  (params (GivenStateList :type "Array of /Game/ProjectCaesar/Blueprints/Enums/ActionStates Enum"))
  (bind _lastactionstates (`self.LastActionStates`))
  (if (not (`self.IsDisabled`))
    (if (>= (`KismetArrayLibrary.Array_Length` (`self.LastActionStates`)) 10)
      (`KismetArrayLibrary.Array_Remove` _lastactionstates))
    (`KismetArrayLibrary.Array_Add` _lastactionstates (`|GetArrayItem` GivenStateList (`KismetArrayLibrary.Array_LastIndex` GivenStateList)))
    (bind _resultvalue (`self.GenerateRatingValue`))
    (`self.ChangeAttentionRating` _resultvalue)))

(event `ChangeAttentionRating`
  (params (ChangeValue :type Integer))
  (bind _returnvalue (+ ChangeValue (`self.AttentionRating`)))
  ;[0.4716 0.724 0.1184] Changes attention rating with input value
  ;;[1 1 1] Clamps values between 0 and 1000 if they exceed those thresholds
  (if (>= _returnvalue 1000)
    (set `self.AttentionRating` 1000)
    (elif (<= _returnvalue 0)
      (set `self.AttentionRating` 0)
      (else
        (set `self.AttentionRating` _returnvalue))))
  (`self.SetAttentionLevelFromRating`))

(event `OnTickMetricEvaluation`
  (`self.NotFightingCheck`))

(event `OnEventMetricEvaluation`)

(event `NotFightingCheck`
  (`KismetSystemLibrary.Delay` 1.0)
  (if (>= (`self.TimeFromLastFight`) (`self.BoredomThresholdSeconds`))
    (`self.ChangeAttentionRating` (* (- (`KismetMathLibrary.FFloor` (`self.BoredomThresholdSeconds`)) (`KismetMathLibrary.FFloor` (`self.TimeFromLastFight`))) 10))))

(event `StopAllTimersAndChecks`
  (set `self.IsDisabled` true))

(fn `DisplayMetricsDebug`
  (`KismetSystemLibrary.PrintString` (`KismetStringLibrary.Concat_StrStr` "Time from Last Kill: " (`KismetStringLibrary.Conv_DoubleToString` (`self.TimeFromLastKill`))) true false (struct :`G` 0.66 :`B` 1.0 :`A` 1.0) 0.01)
  (`KismetSystemLibrary.PrintString` (`KismetStringLibrary.Concat_StrStr` "Time from Last Player Hurt: " (`KismetStringLibrary.Conv_DoubleToString` (`self.TimeFromLastPlayerHurt`))) true false (struct :`G` 0.66 :`B` 1.0 :`A` 1.0) 0.01)
  (`KismetSystemLibrary.PrintString` (`KismetStringLibrary.Concat_StrStr` "Time from Last Fight: " (`KismetStringLibrary.Conv_DoubleToString` (`self.TimeFromLastFight`))) true false (struct :`G` 0.66 :`B` 1.0 :`A` 1.0) 0.01)
  (`KismetSystemLibrary.PrintString` (`KismetStringLibrary.Concat_StrStr` "Time from Last Taunt: " (`KismetStringLibrary.Conv_DoubleToString` (`self.TimeFromLastTaunt`))) true false (struct :`G` 0.66 :`B` 1.0 :`A` 1.0) 0.01)
  (`KismetSystemLibrary.PrintString` (`KismetStringLibrary.Concat_StrStr` "Attention Rating:  " (`KismetStringLibrary.Conv_IntToString` (`self.AttentionRating`))) true false (struct :`G` 0.66 :`B` 1.0 :`A` 1.0) 0.01)
  (`KismetSystemLibrary.PrintString` (`KismetStringLibrary.Concat_StrStr` "Attention Level:  " (`|GetEnumeratorNameAsString` (`self.AttentionLevel`))) true false (struct :`G` 0.66 :`B` 1.0 :`A` 1.0) 0.01)
  (`KismetSystemLibrary.PrintString` (`KismetStringLibrary.Concat_StrStr` "Time from Last Attack: " (`KismetStringLibrary.Conv_DoubleToString` (`self.TimeFromLastAttack`))) true false (struct :`G` 0.66 :`B` 1.0 :`A` 1.0) 0.01))

(fn `GenerateRatingValue`
  (returns (ResultValue :type Integer))
  (locals (RepetitionAmount :type Integer :default -1))
  (bind _lastactionstates (`self.LastActionStates`))
  (bind _lastactionstates_2 (`self.LastActionStates`))
  (for (_ _array_index) (`self.LastActionStates`)
    (if (`|EnumEquality` (`|GetArrayItem` _lastactionstates _array_index) (`|GetArrayItem` _lastactionstates (`KismetArrayLibrary.Array_LastIndex` _lastactionstates)))
      (`/Engine/EditorBlueprintResources/StandardMacros.IncrementInt` (`local.RepetitionAmount`))))
  ;[1 0.1968 0.2366] Returns the value determined by the equation X = Y - (R * D)
  (return (- (`|GetArrayItem` (`self.ActionStateBaseValues`)) (* (`local.RepetitionAmount`) (`|GetArrayItem` (`self.ActionStateDecrementValues`) (`KismetMathLibrary.Conv_ByteToInt` (`|GetArrayItem` _lastactionstates_2 (`KismetArrayLibrary.Array_LastIndex` _lastactionstates_2))))))))

(fn `IncrementAllTimers`
  (params (DeltaSeconds :type "Float (double-precision)"))
  (`self.IncrementTimeFloat` (`self.TimeFromLastKill`) DeltaSeconds)
  (`self.IncrementTimeFloat` (`self.TimeFromLastFight`) DeltaSeconds)
  (`self.IncrementTimeFloat` (`self.TimeFromLastPlayerHurt`) DeltaSeconds)
  (`self.IncrementTimeFloat` (`self.TimeFromLastTaunt`) DeltaSeconds)
  (`self.IncrementTimeFloat` (`self.TimeFromLastAttack`) DeltaSeconds))

(fn `IncrementTimeFloat`
  (params (TimeVariable :type "Float (double-precision) (by ref)") (DeltaTime :type "Float (double-precision)"))
  (`|VariableSetRef` TimeVariable (+ TimeVariable DeltaTime)))

(fn `ResetTimeFloat`
  (params (TimeVariable :type "Float (double-precision) (by ref)"))
  (`|VariableSetRef` TimeVariable))

(fn `SetAttentionLevelFromRating`
  (bind _attentionrating (`self.AttentionRating`))
  (if (< _attentionrating 800)
    (if (< _attentionrating 600)
      (if (< _attentionrating 400)
        (if (< _attentionrating 200)
          (bind _output_get (set `self.AttentionLevel` "NewEnumerator4"))
          (`KismetSystemLibrary.PrintString` (`|GetEnumeratorNameAsString` _output_get))
          (else
            (bind _output_get_2 (set `self.AttentionLevel` "NewEnumerator3"))
            (`KismetSystemLibrary.PrintString` (`|GetEnumeratorNameAsString` _output_get_2))))
        (else
          (bind _output_get_3 (set `self.AttentionLevel` "NewEnumerator2"))
          (`KismetSystemLibrary.PrintString` (`|GetEnumeratorNameAsString` _output_get_3))))
      (else
        (bind _output_get_4 (set `self.AttentionLevel` "NewEnumerator1"))
        (`KismetSystemLibrary.PrintString` (`|GetEnumeratorNameAsString` _output_get_4))))
    (else
      (bind _output_get_5 (set `self.AttentionLevel` "NewEnumerator0"))
      (`KismetSystemLibrary.PrintString` (`|GetEnumeratorNameAsString` _output_get_5))))
  (`KismetSystemLibrary.PrintString` (`KismetStringLibrary.Conv_IntToString` (`self.AttentionRating`))))

(fn `UserConstructionScript`)