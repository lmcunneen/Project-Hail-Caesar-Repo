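; BP_RoundManager runs a gladiatorial round, playing the emperor's intro sequence on BeginPlay and resolving how the round ends.
; CheckIfAllEnemiesAreDead lazily caches all BP_Enemy actors and calls WinSequence once every one is dead.
; WinSequence maxes and stops BP_AttentionMetrics, then compares its average rating to a threshold to play thumbs-up or thumbs-down sequences.
; LoseSequence stops attention tracking and slows global time, with outcomes reported by debug prints.
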(event `self.ReceiveBeginPlay`
  (`MovieSceneSequencePlayer.Play` (`LevelSequenceActor.SequencePlayer` (`self.EmperorStartSequence`))))

(fn `CheckIfAllEnemiesAreDead`
  (if (`KismetArrayLibrary.Array_IsEmpty` (`self.EnemiesList`))
    (bind _outactors (`GameplayStatics.GetAllActorsOfClass` "/Game/ProjectCaesar/Blueprints/BP_Enemy.BP_Enemy_C"))
    (set `self.EnemiesList` _outactors))
  (for _array_element (`self.EnemiesList`)
    (if (not (`/Game/ThirdPerson/Blueprints/BP_ThirdPersonCharacter.IsDead` _array_element))
      (return)))
  (`self.WinSequence`)
  (return))

(fn `LoseSequence`
  (bind _returnvalue (`GameplayStatics.GetActorOfClass` "/Game/ProjectCaesar/Blueprints/BP_AttentionMetrics.BP_AttentionMetrics_C"))
  (`/Game/ProjectCaesar/Blueprints/BP_AttentionMetrics.StopAllTimersAndChecks` _returnvalue)
  (`GameplayStatics.SetGlobalTimeDilation` 0.5)
  (`KismetSystemLibrary.PrintString` "Player Has Lost!" true false (struct :`R` 0.525613 :`G` 0.930092 :`B` 1.0 :`A` 1.0) 100.0))

(fn `UserConstructionScript`)

(fn `WinSequence`
  (`KismetSystemLibrary.PrintString` "All enemies are dead! Playing end sequence" true false (struct :`R` 0.525613 :`G` 0.930092 :`B` 1.0 :`A` 1.0) 100.0)
  (bind _returnvalue (`GameplayStatics.GetActorOfClass` "/Game/ProjectCaesar/Blueprints/BP_AttentionMetrics.BP_AttentionMetrics_C"))
  (set `/Game/ProjectCaesar/Blueprints/BP_AttentionMetrics.AttentionRating` 500 _returnvalue)
  (`/Game/ProjectCaesar/Blueprints/BP_AttentionMetrics.SetAttentionLevelFromRating` _returnvalue)
  (`/Game/ProjectCaesar/Blueprints/BP_AttentionMetrics.StopAllTimersAndChecks` _returnvalue)
  (bind _ratingaverage (`/Game/ProjectCaesar/Blueprints/BP_AttentionMetrics.ReturnAverageRating` _returnvalue))
  (if (>= _ratingaverage (`self.WinThreshold`))
    (`MovieSceneSequencePlayer.Play` (`LevelSequenceActor.SequencePlayer` (`self.ThumbsUpAnim`)))
    (`KismetSystemLibrary.PrintString` "Player has won!" true true (struct :`G` 0.66 :`B` 1.0 :`A` 1.0) 40.0)
    (else
      (`MovieSceneSequencePlayer.Play` (`LevelSequenceActor.SequencePlayer` (`self.ThumbsDownAnim`)))
      (`KismetSystemLibrary.PrintString` "Player has lost!" true true (struct :`G` 0.66 :`B` 1.0 :`A` 1.0) 40.0))))