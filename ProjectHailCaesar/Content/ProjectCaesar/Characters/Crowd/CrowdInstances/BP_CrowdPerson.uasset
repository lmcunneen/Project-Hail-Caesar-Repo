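; BP_CrowdPerson is a modular crowd character that periodically plays paired talking animations with a neighbour.
; Construction makes head, hair and outfit meshes follow the Body's pose via leader pose.
; A person with a valid PersonOnLeftHandSide initiates talks: Tick counts to a random threshold, plays the talk-right montage, then has that neighbour play talk-left.
; When the initiator's montage completes or is interrupted, the timer resets with a new threshold.
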(event `self.ReceiveBeginPlay`
  (if (`KismetSystemLibrary.IsValid` (`self.PersonOnLeftHandSide`))
    (`self.GenerateTalkWaitThreshold`)))

(event `self.ReceiveTick`
  (params (DeltaSeconds :type "Float (single-precision)"))
  (if (`KismetSystemLibrary.IsValid` (`self.PersonOnLeftHandSide`))
    (bind _output_get (set `self.TimeElapsedSinceLastTalk` (+ DeltaSeconds (`self.TimeElapsedSinceLastTalk`))))
    (if (and (>= _output_get (`self.TalkWaitThreshold`)) (not (`self.IsTalking`)))
      (set `self.IsTalking` true)
      (`|PlayMontage` (`self.Body`) "/Game/ProjectCaesar/Characters/Crowd/Animations/AS_CrowdTalkRight_Montage.AS_CrowdTalkRight_Montage"
        (:`then`
          (`self.PlayTalkingAnim` (`self.PersonOnLeftHandSide`)))
        (:`OnCompleted`
          (set `self.TimeElapsedSinceLastTalk` 0.0 :!label _label)
          (`self.GenerateTalkWaitThreshold`)
          (set `self.IsTalking` false))
        (:`OnInterrupted`
          (goto _label))))))

(event `PlayTalkingAnim`
  (`|PlayMontage` (`self.Body`) "/Game/ProjectCaesar/Characters/Crowd/Animations/AS_CrowdTalkLeft_Montage.AS_CrowdTalkLeft_Montage"))

(event `GenerateTalkWaitThreshold`
  (bind _output_get (set `self.TalkWaitThreshold` (`KismetMathLibrary.RandomFloatInRange` 10.0 15.0)))
  (`KismetSystemLibrary.PrintString` (`KismetStringLibrary.Conv_DoubleToString` _output_get) true true (struct :`R` 1.0 :`G` 0.940751 :`A` 1.0)))

(fn `UserConstructionScript`
  ;[0.157 0.599 0.2928] Makes the Modular Skeletal Meshes follow the animation of the Torso Mesh
  (`SkinnedMeshComponent.SetLeaderPoseComponent` (`self.Head`) (`self.Body`) false false)
  (`SkinnedMeshComponent.SetLeaderPoseComponent` (`self.Hair`) (`self.Body`) false false)
  (`SkinnedMeshComponent.SetLeaderPoseComponent` (`self.Outfit`) (`self.Body`) false false))